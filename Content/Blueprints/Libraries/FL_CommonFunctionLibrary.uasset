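; FL_CommonFunctionLibrary is a Blueprint function library of shortcuts to the game's core framework objects.
; It returns the first player's character as BP_FirstPersonCharacter, the game mode as GM_Gameplay and the game instance as GameInst.
; Each getter wraps the engine accessor and a cast, and stops without returning if the cast fails.
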(fn `GetGameInst`
  (returns (`AsGame Inst` :type "/Game/ModesAndStates/GameInst Object Reference"))
  (bind _asgame_inst (cast `/Game/ModesAndStates/GameInst` (`GameplayStatics.GetGameInstance` null)))
  (return _asgame_inst))

(fn `GetGameMode`
  (returns (GMGameplay :type "/Game/ModesAndStates/GM_Gameplay Object Reference"))
  (bind _asgm_gameplay (cast `/Game/ModesAndStates/GM_Gameplay` (`GameplayStatics.GetGameMode` null)))
  (return _asgm_gameplay))

(fn `GetPlayerCharacter`
  (returns (`First Person character Character` :type "/Game/Blueprints/Character/BP_FirstPersonCharacter Object Reference"))
  (bind _asbp_first_person_character (cast `/Game/Blueprints/Character/BP_FirstPersonCharacter` (`GameplayStatics.GetPlayerCharacter` null)))
  (return _asbp_first_person_character))