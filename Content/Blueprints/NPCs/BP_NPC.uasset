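; Interactable NPC that opens a dialogue with the player and can act as a quest giver.
; Interact halts AI logic and movement, then runs a Rotate timeline intended to turn the NPC toward the character.
; When the turn finishes, it creates WB_Dialogue with both names and the dialogue, then disables player look and movement.
; InteractWith delegates to QuestGiverComponent, and a getter exposes CharacterMovement.
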(event `self.ReceiveBeginPlay`
  (bind _asgame_inst (cast `/Game/ModesAndStates/GameInst` (`GameplayStatics.GetGameInstance`)))
  (set `self.As Game Inst` _asgame_inst))

(event `self.ReceiveTick`
  (params (DeltaSeconds :type "Float (single-precision)")))

(event `/Game/Blueprints/Interfaces/BPI_Interaction.Interact`
  (params (CharacterRef :type "/Game/Blueprints/Character/BP_FirstPersonCharacter Object Reference") (PlayerController :type "/Game/ModesAndStates/PC_Gameplay Object Reference"))
  (set `self.Character Ref` CharacterRef)
  (set `self.PlayerControllerRef` PlayerController)
  ; Stops movement and stops them moving immediately
  (message `/Game/Blueprints/Interfaces/BPI_AIController.StopAILogic` (`AIBlueprintHelperLibrary.GetAIController` self) "Started Dialogue")
  (`MovementComponent.StopMovementImmediately` (`self.CharacterMovement`))
  (set `self.PastRotation` (`self.K2_GetActorRotation`))
  ; Rotates the npc towards the character
  (bind (_direction _rotatetrack) (`Timeline|Rotate` :!via `PlayFromStart`)
    (:`Update`
      (bind (_returnvalue_roll _returnvalue_pitch _returnvalue_yaw) (`KismetMathLibrary.BreakRotator` (`KismetMathLibrary.RLerp` (`self.PastRotation`) (`KismetMathLibrary.FindLookAtRotation` (`self.K2_GetActorLocation`) (`self.K2_GetActorLocation`)) _rotatetrack)))
      (`self.K2_SetActorRotation` (`KismetMathLibrary.MakeRotator` _returnvalue_roll 0.0 _returnvalue_yaw)))
    (:`Finished`
      ; Creates dialogue widget and stops the player from moving and looking and shows mouse
      (bind _returnvalue (`|CreateWidget` "/Game/Widgets/WB_Dialogue.WB_Dialogue_C" (`self.PlayerControllerRef`) (`/Game/ModesAndStates/GameInst.PlayerName` (`self.As Game Inst`)) (`self.Name`) (`self.Dialogue`) self))
      (bind _output_get (set `self.DialogueRef` _returnvalue))
      (`UserWidget.AddToViewport` _output_get 0)
      (`/Game/ModesAndStates/PC_Gameplay.DisableLookAndMovement` (`self.PlayerControllerRef`) _returnvalue))))

(fn `GetCharMoveComponent`
  (returns (MovementComponent :type "CharacterMovementComponent Object Reference"))
  (return (`self.CharacterMovement`)))

(fn `InteractWith`
  (returns (ObjectiveID :type String))
  (bind _objectiveid (`/Game/Blueprints/Interfaces/BPI_InteractionV2.InteractWith` (`self.QuestGiverComponent`)))
  (return _objectiveid))

(fn `UserConstructionScript`)