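; BP_NPC_Frog is a frog NPC character Blueprint that waves when the player interacts with it.
; It overrides the inherited Interact event, runs the parent logic, then plays a wave montage on its skeletal mesh.
; All other behavior comes from the parent class, as BeginPlay, overlap and Tick are unused and construction only calls the parent.
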(event `/Game/Blueprints/Interfaces/BPI_Interaction.Interact`
  (params (CharacterRef :type "/Game/Blueprints/Character/BP_FirstPersonCharacter Object Reference") (PlayerController :type "/Game/ModesAndStates/PC_Gameplay Object Reference"))
  (`parent.Interact` CharacterRef PlayerController)
  (`|PlayMontage` (`self.Mesh`) "/Game/Assets/Characters/Frog/Animations/SKM_Frog_Wave_Montage.SKM_Frog_Wave_Montage"))

(fn `UserConstructionScript`
  (`parent.UserConstructionScript`))