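; Swift is an NPC character Blueprint that acts as a quest giver.
; On BeginPlay it fills its QuestGiverComponent's quest data with a row handle to a fixed row in the quest data table.
; Interacting runs the parent behavior, then plays a waving montage on the mesh along with a 2D sound.
; InteractWith forwards to the quest giver component and returns its result.
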(event `self.ReceiveBeginPlay`
  (bind _questgivercomponent (`self.QuestGiverComponent`))
  (`parent.ReceiveBeginPlay`)
  (bind _structout (setmembers `DataTableRowHandle` :`StructRef` (`/Game/Blueprints/QuestSystem/QuestGiverComponent.QuestData` _questgivercomponent) :`DataTable` "/Game/Blueprints/QuestSystem/DTQuestData.DTQuestData" :`RowName` "10001"))
  (set `/Game/Blueprints/QuestSystem/QuestGiverComponent.QuestData` _structout _questgivercomponent))

(event `/Game/Blueprints/Interfaces/BPI_Interaction.Interact`
  (params (CharacterRef :type "/Game/Blueprints/Character/BP_FirstPersonCharacter Object Reference") (PlayerController :type "/Game/ModesAndStates/PC_Gameplay Object Reference"))
  (`parent.Interact` CharacterRef PlayerController)
  (`|PlayMontage` (`self.Mesh`) "/Game/Assets/Characters/Swift/Animations/A_Swift_wave_Montage.A_Swift_wave_Montage"
    (:`then`
      (`GameplayStatics.PlaySound2D` null 1.0 1.0 0.0 null null))))

(fn `InteractWith`
  (returns (ObjectiveID :type String))
  (bind _objectiveid (`/Game/Blueprints/Interfaces/BPI_InteractionV2.InteractWith` (`self.QuestGiverComponent`)))
  (return _objectiveid))

(fn `UserConstructionScript`
  (`parent.UserConstructionScript`))