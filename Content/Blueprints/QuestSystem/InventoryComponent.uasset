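; Inventory component in the quest system that tracks item quantities and reports pickups as objective progress.
; AddToInventory adds the quantity to the item's current count in the Content map, then fires the player character's OnObjectiveIDCalled dispatcher with the item name as objective ID and the added amount as value.
; QueryInventory returns the stored count for an item.
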(fn `AddToInventory`
  (params (Item :type Name) (Quantity :type Integer))
  (`BlueprintMapLibrary.Map_Add` (`self.Content`) Item (+ Quantity (`BlueprintMapLibrary.Map_Find` (`self.Content`) Item)))
  (`/Game/Blueprints/Character/BP_FirstPersonCharacter.OnObjectiveIDCalled` (`/Game/Blueprints/Libraries/FL_CommonFunctionLibrary.GetPlayerCharacter`) (`KismetStringLibrary.Conv_NameToString` (`local.Item`)) (`local.Quantity`)))

(fn `QueryInventory`
  (params (Item :type Name))
  (returns (Value :type Integer))
  (return (`BlueprintMapLibrary.Map_Find` (`self.Content`) Item)))