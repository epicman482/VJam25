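; Quest giver component that offers quests and shows their rewards when the player interacts with its owner.
; InteractWith asks the player's QuestLogComponent about the quest: a new one is either auto-accepted into the log or shown in a WB_QuestGiver widget, per its data table row.
; A completed quest not yet turned in opens WB_QuestRewards instead.
; These interactions return the owner's display name, while LookAt is an empty stub.
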(fn `DisplayQuest`
  (bind (_questdata_datatable _questdata_rowname) (break `DataTableRowHandle` (`self.QuestData`)))
  (bind _returnvalue (`|GetDataTableRow` _questdata_datatable _questdata_rowname)
    (:`then`
      (`KismetSystemLibrary.PrintString` (`KismetStringLibrary.Concat_StrStr` (`KismetTextLibrary.Conv_TextToString` (`.QuestName_2_CA9C3A904E325EBD0F70B48536D7880F` (break `/Game/Blueprints/QuestSystem/FQuestDetails` _returnvalue))) "     QUest name"))
      (bind _returnvalue_2 (`|CreateWidget` "/Game/Widgets/QuestSystem/WB_QuestGiver.WB_QuestGiver_C" null _returnvalue _questdata_rowname))
      (bind _output_get (set `self.QuestGiverRef` _returnvalue_2))
      (`UserWidget.AddToViewport` _output_get 0))))

(fn `DisplayRewards`
  (bind (_questdata_datatable _questdata_rowname) (break `DataTableRowHandle` (`self.QuestData`)))
  (bind _returnvalue (`|GetDataTableRow` "/Game/Blueprints/QuestSystem/DTQuestData.DTQuestData" _questdata_rowname)
    (:`then`
      (bind _returnvalue_2 (`|CreateWidget` "/Game/Widgets/QuestSystem/WB_QuestRewards.WB_QuestRewards_C" null _returnvalue _questdata_rowname))
      (`UserWidget.AddToViewport` _returnvalue_2 0))))

(fn `InteractWith`
  (returns (ObjectiveID :type String))
  (bind (_questdata_datatable _questdata_rowname) (break `DataTableRowHandle` (`self.QuestData`)))
  (bind (_questdata_datatable_2 _questdata_rowname_2) (break `DataTableRowHandle` (`self.QuestData`)))
  (bind (_questdata_datatable_3 _questdata_rowname_3) (break `DataTableRowHandle` (`self.QuestData`)))
  (bind _returnvalue (`Actor.GetComponentByClass` (`GameplayStatics.GetPlayerCharacter` 0) "/Game/Blueprints/QuestSystem/QuestLogComponent.QuestLogComponent_C"))
  (bind _returnvalue_2 (`KismetSystemLibrary.GetDisplayName` (`self.GetOwner`)))
  (bind _questlogcomponent (`/Game/Blueprints/Character/BP_FirstPersonCharacter.QuestLogComponent` (`/Game/Blueprints/Libraries/FL_CommonFunctionLibrary.GetPlayerCharacter`)))
  (if (and (not (`/Game/Blueprints/QuestSystem/QuestLogComponent.QueryActiveQuest` _questlogcomponent _questdata_rowname_2)) (not (`/Game/Blueprints/QuestSystem/QuestLogComponent.QueryCompletedQuests` _questlogcomponent _questdata_rowname_2)))
    (bind _returnvalue_3 (`|GetDataTableRow` "/Game/Blueprints/QuestSystem/DTQuestData.DTQuestData" _questdata_rowname_3)
      (:`then`
        (if (`.AutoAccept_15_75C9D656498542914CC629BECEE186C5` (break `/Game/Blueprints/QuestSystem/FQuestDetails` _returnvalue_3))
          (`/Engine/EditorBlueprintResources/StandardMacros.IsValid` _returnvalue
            (:`Is Valid`
              (`/Game/Blueprints/QuestSystem/QuestLogComponent.AddNewQuest` _returnvalue _questdata_rowname_3)
              (return _returnvalue_2)))
          (else
            (`self.DisplayQuest`)
            (return _returnvalue_2)))))
    (else
      (bind _questactor (`/Game/Blueprints/QuestSystem/QuestLogComponent.GetQuestActor` (`/Game/Blueprints/Character/BP_FirstPersonCharacter.QuestLogComponent` (`/Game/Blueprints/Libraries/FL_CommonFunctionLibrary.GetPlayerCharacter`)) _questdata_rowname))
      (if (and (`/Game/Blueprints/QuestSystem/Quest_Base.IsCompleted` _questactor) (not (`/Game/Blueprints/QuestSystem/Quest_Base.IsTurnedIn` _questactor)))
        (`self.DisplayRewards`)
        (return _returnvalue_2)))))

(fn `LookAt`
  (return))