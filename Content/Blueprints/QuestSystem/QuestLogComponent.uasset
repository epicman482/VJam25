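; Quest log component that records active and completed quests by ID and handles adding, querying, tracking and turning them in.
; Each new quest spawns a Quest_Base actor, which is later looked up by ID.
; Turn-in only prints the stage's XP reward, then completes the quest, flagging its actor and firing OnQuestCompleted.
; Tracking creates a single WB_Tracker widget on first use and updates it afterwards.
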(fn `AddNewQuest`
  (params (QuestID :type Name))
  (returns (ReturnValue :type "/Game/Blueprints/QuestSystem/Quest_Base Object Reference"))
  (`KismetArrayLibrary.Array_AddUnique` (`self.CurrentActiveQuests`) QuestID)
  (bind _returnvalue (`|SpawnActorFromClass` "/Game/Blueprints/QuestSystem/Quest_Base.Quest_Base_C" (`KismetMathLibrary.MakeTransform` (0.0 0.0 0.0)) "Undefined" "MultiplyWithRoot" null QuestID null))
  (`KismetArrayLibrary.Array_Add` (`self.CurrentQuests`) _returnvalue)
  (return _returnvalue))

(fn `CompleteQuest`
  (params (QuestID :type Name))
  (bind _questid (`local.QuestID`))
  (`KismetArrayLibrary.Array_AddUnique` (`self.CompleatedQuests`) QuestID)
  (`KismetArrayLibrary.Array_RemoveItem` (`self.CurrentActiveQuests`) _questid)
  (bind _questactor (`self.GetQuestActor` _questid))
  (set `/Game/Blueprints/QuestSystem/Quest_Base.IsTurnedIn` true _questactor)
  (`self.OnQuestCompleted` _questactor))

(fn `GetQuestActor`
  (params (QuestID :type Name))
  (returns (QuestActor :type "/Game/Blueprints/QuestSystem/Quest_Base Object Reference"))
  (for _array_element (`self.CurrentQuests`)
    (if (== (`/Game/Blueprints/QuestSystem/Quest_Base.QuestID` _array_element) QuestID)
      (return _array_element))))

(fn `QueryActiveQuest`
  (params (QuestID :type Name))
  (returns (ReturnValue :type Boolean))
  (return (`KismetArrayLibrary.Array_Contains` (`self.CurrentActiveQuests`) QuestID)))

(fn `QueryCompletedQuests`
  (params (QuestID :type Name))
  (returns (ReturnValue :type Boolean) (TurnedIn :type Boolean))
  (bind _returnvalue (`KismetArrayLibrary.Array_Contains` (`self.CompleatedQuests`) QuestID))
  (bind _questactor (`self.GetQuestActor` QuestID))
  (`/Engine/EditorBlueprintResources/StandardMacros.IsValid` _questactor
    (:`Is Valid`
      (return _returnvalue (`/Game/Blueprints/QuestSystem/Quest_Base.IsTurnedIn` _questactor)))
    (:`Is Not Valid`
      (return _returnvalue true))))

(fn `TrackQuest`
  (params (QuestActor :type "/Game/Blueprints/QuestSystem/Quest_Base Object Reference"))
  (bind _tracker (`self.Tracker`)
    (:`then`
      (`/Game/Widgets/QuestSystem/WB_Tracker.Update` _tracker QuestActor))
    (:`else`
      (bind _returnvalue (`|CreateWidget` "/Game/Widgets/QuestSystem/WB_Tracker.WB_Tracker_C" null QuestActor))
      (bind _output_get (set `self.Tracker` _returnvalue))
      (`UserWidget.AddToViewport` _output_get -1))))

(fn `TurnInQuest`
  (params (QuestID :type Name))
  (`|ExecutionSequence`
    (:`then_0`
      (bind _questactor (`self.GetQuestActor` QuestID))
      (`KismetSystemLibrary.PrintString` (`KismetTextLibrary.Conv_TextToString` (`|FormatText` "XP = {a}" (`.XPReward_9_A1D9A436460719B79380F3A5782722B2` (break `/Game/Blueprints/QuestSystem/FStageDetails` (`/Game/Blueprints/QuestSystem/Quest_Base.CurrentStageDetails` _questactor)))))))
    (:`then_1`
      (`self.CompleteQuest` QuestID))))