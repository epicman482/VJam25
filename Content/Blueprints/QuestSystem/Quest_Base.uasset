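; Base quest actor that loads its quest data from a data table and tracks objective progress for the current stage.
; On BeginPlay it seeds a progress map, subscribes to the player's objective-ID event and pre-counts one objective type from the inventory.
; Heard IDs adjust progress, with increases applied only below the required quantity.
; Reaching that quantity shows a quest notification widget with the objective's description.
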(event `self.ReceiveBeginPlay`
  (`self.GetQuestDetails`)
  (add `/Game/Blueprints/Character/BP_FirstPersonCharacter.OnObjectiveIDCalled` (`/Game/Blueprints/Libraries/FL_CommonFunctionLibrary.GetPlayerCharacter`) (`|CreateDelegate` :!event `OnObjectiveIDHeard`))
  (for _array_element (`.Objectives_20_6C63776144E0C7074EC1238A47FD9DE5` (break `/Game/Blueprints/QuestSystem/FStageDetails` (`self.CurrentStageDetails`)))
    (bind ((`Type_20_C150A64741FFD8D15D5F62940BA93FD2` _type) (`ObjectiveID_10_9A6F4BB14C91DDCAED0085A59A45B89D` _objectiveid)) (break `/Game/Blueprints/QuestSystem/FObjectiveDetails` _array_element))
    (if (`|EnumEquality` _type "NewEnumerator2")
      (bind _value (`/Game/Blueprints/QuestSystem/InventoryComponent.QueryInventory` (`/Game/Blueprints/Character/BP_FirstPersonCharacter.InventoryComponent` (`/Game/Blueprints/Libraries/FL_CommonFunctionLibrary.GetPlayerCharacter`)) (`KismetStringLibrary.Conv_StringToName` _objectiveid)))
      (`self.OnObjectiveIDHeard` _objectiveid _value))))

(fn `GetObjectiveDataByID`
  (params (ObjectiveID :type String))
  (returns (`Array Element` :type "/Game/Blueprints/QuestSystem/FObjectiveDetails Structure"))
  (for _array_element (`.Objectives_20_6C63776144E0C7074EC1238A47FD9DE5` (break `/Game/Blueprints/QuestSystem/FStageDetails` (`self.CurrentStageDetails`)))
    (if (`KismetStringLibrary.EqualEqual_StrStr` (`.ObjectiveID_10_9A6F4BB14C91DDCAED0085A59A45B89D` (break `/Game/Blueprints/QuestSystem/FObjectiveDetails` _array_element)) ObjectiveID)
      (return _array_element))))

(fn `GetQuestDetails`
  (bind _returnvalue (`|GetDataTableRow` "/Game/Blueprints/QuestSystem/DTQuestData.DTQuestData" (`self.QuestID`))
    (:`then`
      (bind _output_get (set `self.QuestDetails` _returnvalue))
      (bind _output_get_2 (set `self.CurrentStageDetails` (`|GetArrayItem` (`.Stages_13_E07811D047DF32C387A95D8C0375BBD4` (break `/Game/Blueprints/QuestSystem/FQuestDetails` _output_get)) (`self.CurrentStage`))))
      (`BlueprintMapLibrary.Map_Clear` (`self.CurrentObjectiveProgress`))
      (for _array_element (`.Objectives_20_6C63776144E0C7074EC1238A47FD9DE5` (break `/Game/Blueprints/QuestSystem/FStageDetails` _output_get_2))
        (`BlueprintMapLibrary.Map_Add` (`self.CurrentObjectiveProgress`) (`.ObjectiveID_10_9A6F4BB14C91DDCAED0085A59A45B89D` (break `/Game/Blueprints/QuestSystem/FObjectiveDetails` _array_element)))))))

(fn `IsObjectiveComplete`
  (params (ObjectiveID :type String))
  (bind ((`Description_4_65D14FA841F30B5160F7E981ACFF9CA4` _description) (`Quantity_13_0259375347C76BD81FC7839EF6D765B4` _quantity)) (break `/Game/Blueprints/QuestSystem/FObjectiveDetails` (`self.GetObjectiveDataByID` ObjectiveID)))
  (if (>= (`BlueprintMapLibrary.Map_Find` (`self.CurrentObjectiveProgress`) (`local.ObjectiveID`)) _quantity)
    (bind _returnvalue (`|CreateWidget` "/Game/Widgets/QuestSystem/WB_QuestNotification.WB_QuestNotification_C" null _description))
    (`UserWidget.AddToViewport` _returnvalue 0)))

(fn `OnObjectiveIDHeard`
  (params (ObjectiveID :type String) (Value :type Integer :default 1))
  (bind _objectiveid (`local.ObjectiveID`))
  (bind (_value _returnvalue) (`BlueprintMapLibrary.Map_Find` (`self.CurrentObjectiveProgress`) (`local.ObjectiveID`)))
  (if (> (`KismetMathLibrary.SignOfInteger` Value) 0)
    (if _returnvalue
      (if (< _value (`.Quantity_13_0259375347C76BD81FC7839EF6D765B4` (break `/Game/Blueprints/QuestSystem/FObjectiveDetails` (`self.GetObjectiveDataByID` (`local.ObjectiveID`)))))
        (`BlueprintMapLibrary.Map_Add` (`self.CurrentObjectiveProgress`) _objectiveid (+ _value (`local.Value`)))
        (`self.IsObjectiveComplete` _objectiveid)
        (return))
      (else
        (return)))
    (else
      (`BlueprintMapLibrary.Map_Add` (`self.CurrentObjectiveProgress`) (`local.ObjectiveID`) (+ (`BlueprintMapLibrary.Map_Find` (`self.CurrentObjectiveProgress`) (`local.ObjectiveID`)) (`local.Value`)))
      (return))))

(fn `UserConstructionScript`)