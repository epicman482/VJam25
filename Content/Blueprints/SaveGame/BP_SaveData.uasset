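; BP_SaveData stores quest state for saving: active and completed quest lists, plus a progress map keyed by quest ID.
; SaveQuestLog copies both lists from a quest log, while SaveQuestDetails records one quest's current stage and objective progress in the map.
; LoadQuests re-adds each active quest to the log, restores its stage and progress from the map, then overwrites the log's two lists with the saved ones.
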(fn `LoadQuests`
  (params (`Quest Log` :type "/Game/Blueprints/QuestSystem/QuestLogComponent Object Reference"))
  (for _array_element (`self.CurrentActiveQuests`)
    (bind _returnvalue (`/Game/Blueprints/QuestSystem/QuestLogComponent.AddNewQuest` `Quest Log` _array_element))
    (bind (_progress _currentstage) (break `/Game/Blueprints/QuestSystem/FQuestSaveData` (`BlueprintMapLibrary.Map_Find` (`self.QuestProgress`) _array_element)))
    (set `/Game/Blueprints/QuestSystem/Quest_Base.CurrentStage` _currentstage _returnvalue)
    (set `/Game/Blueprints/QuestSystem/Quest_Base.CurrentObjectiveProgress` _progress _returnvalue))
  (set `/Game/Blueprints/QuestSystem/QuestLogComponent.CurrentActiveQuests` (`self.CurrentActiveQuests`) `Quest Log`)
  (set `/Game/Blueprints/QuestSystem/QuestLogComponent.CompleatedQuests` (`self.CompletedQuests`) `Quest Log`))

(fn `SaveQuestDetails`
  (params (Quest :type "/Game/Blueprints/QuestSystem/Quest_Base Object Reference"))
  (`BlueprintMapLibrary.Map_Add` (`self.QuestProgress`) (`/Game/Blueprints/QuestSystem/Quest_Base.QuestID` Quest) (make `/Game/Blueprints/QuestSystem/FQuestSaveData` (`/Game/Blueprints/QuestSystem/Quest_Base.CurrentObjectiveProgress` Quest) (`/Game/Blueprints/QuestSystem/Quest_Base.CurrentStage` Quest))))

(fn `SaveQuestLog`
  (params (QuestLog :type "/Game/Blueprints/QuestSystem/QuestLogComponent Object Reference"))
  (set `self.CurrentActiveQuests` (`/Game/Blueprints/QuestSystem/QuestLogComponent.CurrentActiveQuests` QuestLog))
  (set `self.CompletedQuests` (`/Game/Blueprints/QuestSystem/QuestLogComponent.CompleatedQuests` QuestLog)))