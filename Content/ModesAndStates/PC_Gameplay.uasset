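; PC_Gameplay is the player controller that boots the game's front end and toggles player control between UI and gameplay.
; On BeginPlay it sets windowed fullscreen, plays the music track, and stacks a splash widget over the main menu with the mouse cursor shown.
; Two custom events disable or restore move and look input on player 0, switching cursor visibility and input mode between Game-and-UI and Game-only.
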(event `self.ReceiveBeginPlay`
  (bind _returnvalue (`GameUserSettings.GetGameUserSettings`))
  (`GameUserSettings.SetFullscreenMode` _returnvalue "WindowedFullscreen")
  (if true
    (`GameplayStatics.PlaySound2D` "/Game/Audio/deraj_-_REWILD_GJ_2025.deraj_-_REWILD_GJ_2025" 1.0 1.0 0.0 null null)
    (bind _returnvalue_2 (`|CreateWidget` "/Game/Widgets/WB_Splash.WB_Splash_C"))
    (`UserWidget.AddToViewport` _returnvalue_2 99)
    (set `self.bShowMouseCursor` true)
    (bind _returnvalue_3 (`|CreateWidget` "/Game/Widgets/WB_MainMenu.WB_MainMenu_C"))
    (`UserWidget.AddToViewport` _returnvalue_3 0)
    (`WidgetBlueprintLibrary.SetInputMode_GameAndUIEx` self _returnvalue_3)))

(event `DisableLookAndMovement`
  (params (InWidgetToFocus :type "Widget Object Reference"))
  (bind _returnvalue (`GameplayStatics.GetPlayerController` 0))
  (`self.SetIgnoreMoveInput` _returnvalue true)
  (`self.SetIgnoreLookInput` _returnvalue true)
  (set `PlayerController.bShowMouseCursor` true _returnvalue)
  (`WidgetBlueprintLibrary.SetInputMode_GameAndUIEx` _returnvalue InWidgetToFocus "DoNotLock" false))

(event `EnableLookAndMovement`
  (bind _returnvalue (`GameplayStatics.GetPlayerController` 0))
  (`self.ResetIgnoreMoveInput` _returnvalue)
  (`self.ResetIgnoreLookInput` _returnvalue)
  (set `PlayerController.bShowMouseCursor` false _returnvalue)
  (`WidgetBlueprintLibrary.SetInputMode_GameOnly` _returnvalue))

(fn `UserConstructionScript`)